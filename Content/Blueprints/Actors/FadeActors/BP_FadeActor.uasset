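; BP_FadeActor is an actor whose mesh fades out and back in on request.
; Construction caches the original materials and builds dynamic instances from fade materials, which FadeOut swaps onto the mesh by slot index.
; One timeline drives their "Fade" parameter, playing for FadeOut and reversing for Fadein.
; When finished, fully faded meshes ignore a custom trace channel (optionally Visibility), while restored ones block again with original materials.
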(event EventFadein
  (bind _fadeouttimeline (Timeline|FadeTimeline Reverse)
    (:Update
      (for _array_element (Variables|Default|GetDynamicMaterialInstances)
        (Rendering|Material|SetScalarParameterValue _array_element "Fade" _fadeouttimeline :!class /Script/Engine.MaterialInstanceDynamic)))
    (:Finished
      (CallFunction|FadeFinished _fadeouttimeline))))

(event EventFadeOut
  (CallFunction|SetMaterialtoDynamicInstances)
  (bind _fadeouttimeline (Timeline|FadeTimeline Play)
    (:Update
      (for _array_element (Variables|Default|GetDynamicMaterialInstances)
        (Rendering|Material|SetScalarParameterValue _array_element "Fade" _fadeouttimeline :!class /Script/Engine.MaterialInstanceDynamic)))
    (:Finished
      (CallFunction|FadeFinished _fadeouttimeline))))

(fn ConstructionScript
  (Utilities|Array|Clear (Variables|Default|GetDynamicMaterialInstances))
  (Variables|Default|SetOriginalMateerials (Rendering|Material|GetMaterials (Variables|Default|GetMesh)))
  (for _array_element (Variables|Default|GetFadeMaterialInstances)
    (bind _returnvalue (Rendering|Material|CreateDynamicMaterialInstance _array_element "None" "None" :!class /Script/Engine.KismetMaterialLibrary))
    (Utilities|Array|AddUnique (Variables|Default|GetDynamicMaterialInstances) _returnvalue)))

(fn SetMaterialtoDynamicInstances
  (for (_array_element _array_index) (Variables|Default|GetDynamicMaterialInstances)
    (Rendering|Material|SetMaterial (Variables|Default|GetMesh) _array_index _array_element)))

(fn ResetMaterials
  (for (_array_element _array_index) (Variables|Default|GetOriginalMateerials)
    (Rendering|Material|SetMaterial (Variables|Default|GetMesh) _array_index _array_element)))

(fn FadeFinished
  (params (InputPin :type Float%20%28single-precision%29))
  (if (>= InputPin 1.0)
    (CallFunction|ResetMaterials)
    (Collision|SetCollisionResponsetoChannel (Variables|Default|GetMesh) "ECC_GameTraceChannel3" "ECR_Block")
    (if (Variables|Default|GetBlockVisibility)
      (Collision|SetCollisionResponsetoChannel (Variables|Default|GetMesh) "ECC_Visibility" "ECR_Block"))
    (elif (<= InputPin 0.0)
      (Collision|SetCollisionResponsetoChannel (Variables|Default|GetMesh) "ECC_GameTraceChannel3" "ECR_Ignore")
      (if (Variables|Default|GetBlockVisibility)
        (Collision|SetCollisionResponsetoChannel (Variables|Default|GetMesh) "ECC_Visibility" "ECR_Ignore")))))