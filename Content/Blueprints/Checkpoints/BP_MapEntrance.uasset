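; BP_MapEntrance is a map entrance actor, filed with the checkpoints, that lights up when highlighted.
; It overrides the inherited HighlightActor and UnHighlightActor events, calling the parent first and then showing or hiding its eight point lights without propagating to children.
; It has no other active logic: BeginPlay and Tick are disabled and the construction script is empty.
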(event EventBeginPlay)

(event EventTick
  (params (DeltaSeconds :type Float%20%28single-precision%29)))

(event EventHighlightActor
  (|CallParentFunction)
  (Rendering|SetVisibility (Variables|Default|GetPointLight1) true false))

(event EventUnHighlightActor
  (|CallParentFunction)
  (Rendering|SetVisibility (Variables|Default|GetPointLight1) false false))

(fn ConstructionScript)