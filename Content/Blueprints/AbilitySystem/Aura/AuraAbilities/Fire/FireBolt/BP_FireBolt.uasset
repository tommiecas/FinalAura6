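; BP_FireBolt is the fire bolt actor for the Aura Fire Bolt ability.
; On BeginPlay it waits briefly, then enables query-only collision on its Sphere.
; Each tick MakeGoKaboomIfNoGo records the current and previous locations.
; Its stall check, meant to play impact sound and explosion then destroy the actor, is disconnected, as is a debug sphere draw.
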(event EventTick
  (params (DeltaSeconds :type Float%20%28single-precision%29))
  (CallFunction|MakeGoKaboomifNoGo))

(event Collision|EventActorBeginOverlap
  (params (OtherActor :type Actor%20Object%20Reference)))

(event EventBeginPlay
  (Utilities|FlowControl|Delay 0.5)
  (bind _sphere (Variables|Default|GetSphere)
    (:then
      (Collision|SetCollisionEnabled _sphere "QueryOnly"))
    (:else)))

(fn ConstructionScript)

(fn MakeGoKaboomifNoGo
  (Variables|Default|SetLocationLastFrame (Variables|Default|GetLocationThisFrame))
  (Variables|Default|SetLocationThisFrame (Transformation|GetActorLocation)))