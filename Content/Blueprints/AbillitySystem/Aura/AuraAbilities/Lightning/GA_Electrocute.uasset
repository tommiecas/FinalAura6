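; Electrocute lightning ability for the Aura character that holds the avatar in a shock loop while the input is held.
; It stores the mouse hit, turns the avatar toward it and plays a montage whose gameplay event starts the loop and disables movement.
; Releasing the input clears the loop, restores walking and ends the ability.
; Avatar calls go through CombatInterface, checked on activation; no damage or targeting beam is handled here.
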(event Ability|EventActivateAbility
  (CallFunction|VerifyCombatInterfaceImplementation)
  ;[1 0.2517 0.7046] Store Mouse Data Variables
  (bind _datahandle (|TargetDataUnderMouse)
    (:ValidData
      (Class|AuraBeamSpell|StoreMouseDataInfo (Ability|TargetData|GetHitResultfromTargetData _datahandle))
      (Class|AuraBeamSpell|StoreOwnerVariables)
      (Utilities|FlowControl|Sequence
        (:then_0
          (Variables|/Script/Engine.PlayerController|SetbShowMouseCursor (Variables|Default|GetOwnerPlayerController) false)
          (CallFunction|UpdatingFacingTarget)
          (|PlayMontageandWaitProxy "None" (Variables|Default|GetElectrocuteMontage) 1.0 "None" false 1.0 0.0 false
            (:then
              (Ability|Tasks|WaitGameplayEvent "(TagName=\"Event.Montage.Electrocute\")" 0 true
                (:EventReceived
                  (CallFunction|InShockLoop))))))
        (:then_1
          (Ability|Tasks|WaitInputRelease false
            (:OnRelease
              (CallFunction|PreparetoEndAbility)
              (Ability|EndAbility))))))))

(fn VerifyCombatInterfaceImplementation
  (if (not (Utilities|DoesObjectImplementInterface (Ability|GetAvatarActorfromActorInfo) "/Script/Aura.CombatInterface"))
    (Ability|EndAbility)))

(fn PreparetoEndAbility
  (Variables|/Script/Engine.PlayerController|SetbShowMouseCursor (Variables|Default|GetOwnerPlayerController) false)
  (Class|CombatInterface|SetinShockLoop(Message) (Ability|GetAvatarActorfromActorInfo) false)
  (Pawn|Components|CharacterMovement|SetMovementMode (Variables|/Script/Engine.Character|GetCharacterMovement (Variables|Default|GetOwnerCharacter)) "MOVE_Walking" 0))

(fn InShockLoop
  (Class|CombatInterface|SetinShockLoop(Message) (Ability|GetAvatarActorfromActorInfo) true)
  (Pawn|Components|CharacterMovement|DisableMovement (Variables|/Script/Engine.Character|GetCharacterMovement (Variables|Default|GetOwnerCharacter))))

(fn UpdatingFacingTarget
  (Class|CombatInterface|UpdateFacingTarget(Message) (Ability|GetAvatarActorfromActorInfo) (Variables|Default|GetMouseHitLocation)))